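; 2D sprite lift that shuttles between its origin and EndLocation, with configurable color and travel time.
; A timeline lerps the Lift's relative location; on finishing, it waits StopDelay and runs in the opposite direction.
; A SafetyCollider overlap by MyCharacter calls Play or Reverse on an active timeline, depending on its playing state.
; The construction script tints the sprite and uses TestEndLocation to place it at either endpoint.
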(event `self.ReceiveBeginPlay`
  (`TimelineComponent.SetPlayRate` (`self.LiftTimeline`) (/ 1.0 (`self.TravelTimeInSeconds`)))
  (set `self.TestEndLocation` true))

(event `self.SafetyCollider.OnComponentBeginOverlap`
  (params (OverlappedComponent :type "PrimitiveComponent Object Reference") (OtherActor :type "Actor Object Reference") (OtherComp :type "PrimitiveComponent Object Reference") (OtherBodyIndex :type Integer) (bFromSweep :type Boolean) (SweepResult :type "HitResult Structure (by ref)"))
  (bind _lifttimeline (`self.LiftTimeline`))
  (cast `/Game/Blueprints/MyCharacter` OtherActor)
  (if (`ActorComponent.IsActive` _lifttimeline)
    (if (`TimelineComponent.IsPlaying` _lifttimeline)
      (bind (_direction _mydriver) (`Timeline|LiftTimeline` :!label _label)
        (:`Update`
          (`SceneComponent.K2_SetRelativeLocation` (`self.Lift`) (`KismetMathLibrary.VLerp` (0.0 0.0 0.0) (`self.EndLocation`) _mydriver) false false))
        (:`Finished`
          (`KismetSystemLibrary.Delay` (`self.StopDelay`))
          (switch `ETimelineDirection` _direction
            (:`Forward`
              (`self.LiftBackward`))
            (:`Backward`
              (`self.LiftFoward`)))))
      (else
        (goto _label :!via `Reverse`)))))

(event `LiftFoward`
  (goto _label :!via `PlayFromStart`))

(event `LiftBackward`
  (goto _label :!via `ReverseFromEnd`))

(fn `UserConstructionScript`
  (bind _lift (`self.Lift`))
  (`SceneComponent.K2_SetRelativeLocation` _lift (`KismetMathLibrary.SelectVector` (`self.EndLocation`) (0.0 0.0 0.0) (`self.TestEndLocation`)) false false)
  (`PaperSpriteComponent.SetSpriteColor` _lift (`self.LiftColor`)))