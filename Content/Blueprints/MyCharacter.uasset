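; MyCharacter is a 2D side-scrolling flipbook character that runs along the X axis and jumps.
; The MoveRight axis event applies movement, yaws the controller to 0 or 180 to face the travel direction, and calls UpdateAnimation.
; UpdateAnimation feeds velocity and falling state into AnimationStateMachine, which selects the Idle, Running or Jumping flipbook for the Sprite.
; Tick is unused, and the Sprite is set to replicate on BeginPlay.
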(event `self.ReceiveBeginPlay`
  (`ActorComponent.SetIsReplicated` (`self.Sprite`) true))

(event `InputAxis|MoveRight`
  (params (AxisValue :type "Float (single-precision)"))
  (`self.AddMovementInput` (1.0 0.0 0.0) AxisValue)
  (`self.Update Animation`)
  (`/Engine/EditorBlueprintResources/StandardMacros.CompareFloat` AxisValue
    (:`>`
      (`Controller.SetControlRotation` (`self.GetController`) (`KismetMathLibrary.MakeRotator` 0.0)))
    (:`<`
      (`Controller.SetControlRotation` (`self.GetController`) (`KismetMathLibrary.MakeRotator` 0.0 0.0 180.0)))))

(event `InputAction|Jump`
  (params (Key :type "Key Structure"))
  (:`Pressed`
    (`self.Jump`)))

(event `Update Animation`
  (set `self.isMoving` (> (`KismetMathLibrary.VSize` (`self.GetVelocity`)) 0.0))
  (set `self.isFalling` (`NavMovementComponent.IsFalling` (`self.CharacterMovement`)))
  (bind _outputflipbook (`self.Animation State Machine` (`self.isFalling`) (`self.isMoving`)))
  (`PaperFlipbookComponent.SetFlipbook` (`self.Sprite`) _outputflipbook))

(fn `Animation State Machine`
  (params (isFalling :type Boolean) (isMoving :type Boolean))
  (returns (outputFlipbook :type "PaperFlipbook Object Reference"))
  (locals (AnimationState :type "/Game/Data/AnimationState Enum") (isFallingLocal :type Boolean) (isMovingLocal :type Boolean))
  (set `local.isFallingLocal` isFalling)
  (set `local.isMovingLocal` isMoving)
  (if (`local.isFallingLocal`)
    (set `local.AnimationState` "NewEnumerator2")
    (elif (`local.isMovingLocal`)
      (set `local.AnimationState` "NewEnumerator1")
      (else
        (set `local.AnimationState` "NewEnumerator0"))))
  (return (select `/Game/Data/AnimationState` (`local.AnimationState`) :`NewEnumerator0` (`self.IdleFlipbook`) :`NewEnumerator1` (`self.runFlipbook`) :`NewEnumerator2` (`self.jumpFlipbook`))))

(fn `UserConstructionScript`)